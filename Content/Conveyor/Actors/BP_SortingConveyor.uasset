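; Conveyor actor that runs only in response to actors overlapping its Box, presumably for a sorting line.
; Each Tick polls the Box overlaps and calls SetMoving at a fixed speed for any actor that is not an FPS_VRCharacter.
; It calls StopMoving only when the Box is completely empty, so a player standing alone in it leaves the current state unchanged.
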(event `self.ReceiveTick`
  (params (DeltaSeconds :type "Float (single-precision)"))
  (bind _overlappingactors (`PrimitiveComponent.GetOverlappingActors` (`self.Box`) null))
  (`parent.ReceiveTick` DeltaSeconds)
  (if (> (`KismetArrayLibrary.Array_Length` _overlappingactors) 0)
    (for _array_element _overlappingactors
      (cast `/Game/VRE/Core/Character/FPS_VRCharacter` _array_element
        (:`CastFailed`
          (`self.SetMoving` 100.0))))
    (else
      (`self.StopMoving`))))

(fn `UserConstructionScript`
  (`parent.UserConstructionScript`))