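; BP_UIActor tracks score and missed score for the Conveyor game and displays them through a widget.
; AddScore and AddMissedScore increment their counters and push the values to BP_ScoreUI, obtained from the Widget.
; When Score reaches MaxScore, AddScore reopens the Conveyor level, then calls the Spawner's ChangePair if Score is a multiple of ChangeObjectInterval.
; That interval check runs only inside the max-score branch.
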(event `AddScore`
  (bind _output_get (set `self.Score` (+ (`self.Score`) 1)))
  (bind _asbp_score_ui (cast `/Game/Conveyor/Actors/BP_ScoreUI` (`WidgetComponent.GetWidget` (`self.Widget`))))
  (`/Game/Conveyor/Actors/BP_ScoreUI.UpdateScore` _asbp_score_ui _output_get)
  (if (>= (`self.Score`) (`self.MaxScore`))
    (`GameplayStatics.OpenLevel` "Conveyor")
    (if (== (mod (`self.Score`) (`self.ChangeObjectInterval`)) 0)
      (`/Game/Conveyor/Actors/BP_ObjectSpawner.ChangePair` (`self.Spawner`)))))

(event `AddMissedScore`
  (bind _result (`/Engine/EditorBlueprintResources/StandardMacros.IncrementInt` (`self.MissedScore`))
    (:`  `
      (bind _asbp_score_ui (cast `/Game/Conveyor/Actors/BP_ScoreUI` (`WidgetComponent.GetWidget` (`self.Widget`))))
      (`/Game/Conveyor/Actors/BP_ScoreUI.UpdateMissedScore` _asbp_score_ui _result))))

(fn `UserConstructionScript`)