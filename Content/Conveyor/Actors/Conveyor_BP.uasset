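; Conveyor belt actor that carries any actors overlapping its Box component along the belt's direction.
; Each Tick it offsets those actors along the static mesh's forward vector by Speed times delta time, without sweeping.
; The construction script creates a dynamic instance of Conveyor_M and feeds it color, X scale and a TrackSpeed scroll value, which is set separately from the push Speed.
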(event `self.ReceiveTick`
  (params (DeltaSeconds :type "Float (single-precision)"))
  (for _array_element (`PrimitiveComponent.GetOverlappingActors` (`self.Box`) null)
    (`self.K2_AddActorWorldOffset` _array_element (* (* DeltaSeconds (`self.Speed`)) (`KismetMathLibrary.GetForwardVector` (`SceneComponent.K2_GetComponentRotation` (`self.StaticMesh`)))) false false)))

(fn `UserConstructionScript`
  (bind _returnvalue (`PrimitiveComponent.CreateDynamicMaterialInstance` (`self.StaticMesh`) 0 "/Game/Conveyor/Materials/Conveyor_M.Conveyor_M" "None"))
  (`MaterialInstanceDynamic.SetVectorParameterValue` _returnvalue "Color" (`self.Color`))
  (`MaterialInstanceDynamic.SetScalarParameterValue` _returnvalue "XScale" (`self.Scale`))
  (`MaterialInstanceDynamic.SetScalarParameterValue` _returnvalue "XSpeed" (`self.TrackSpeed`)))