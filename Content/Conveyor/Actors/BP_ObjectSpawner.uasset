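; Conveyor object spawner actor that spawns good and bad items at its own transform on a looping timer started at BeginPlay.
; Each tick of the timer increments a counter and spawns a bad item when it is a multiple of BadItemSpawnPeriod, otherwise a good item.
; Both classes come from parallel arrays indexed by PairIndex, which the ChangePair event cycles with wraparound.
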(event `self.ReceiveBeginPlay`
  (`self.StartTimer`))

(event `StartTimer`
  (bind _returnvalue (`self.GetTransform`))
  (`KismetSystemLibrary.K2_SetTimerDelegate` (delegate `Delta1Second`) (`self.SpawnInterval`) true)
  (`KismetSystemLibrary.PrintString` (`KismetStringLibrary.Conv_IntToString` (stale `Delta1Second` _result)) :!label _label)
  (if (== (mod (`self.Time`) (`self.BadItemSpawnPeriod`)) 0)
    (`|SpawnActorFromClass` (`|GetArrayItem` (`self.BadItem`) (`self.PairIndex`)) _returnvalue "Undefined" "MultiplyWithRoot" null null)
    (`KismetSystemLibrary.PrintString` (`KismetStringLibrary.Conv_IntToString` (`self.PairIndex`)))
    (else
      (`|SpawnActorFromClass` (`|GetArrayItem` (`self.GoodItem`) (`self.PairIndex`)) _returnvalue "Undefined" "MultiplyWithRoot" null null))))

(event `Delta1Second`
  (bind _result (`/Engine/EditorBlueprintResources/StandardMacros.IncrementInt` (`self.Time`))
    (:`  `
      (goto _label))))

(event `ChangePair`
  (bind _pairindex (`self.PairIndex`))
  (if (>= _pairindex (- (`KismetArrayLibrary.Array_Length` (`self.GoodItem`)) 1))
    (set `self.PairIndex` 0)
    (else
      (`/Engine/EditorBlueprintResources/StandardMacros.IncrementInt` _pairindex))))

(fn `UserConstructionScript`)