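; BP_Conveyor is a conveyor belt actor that carries overlapping actors along its surface.
; Each tick it offsets every actor inside its Box, except FPS_VRCharacter, along the mesh's forward vector at Speed, without sweep or physics forces.
; The construction script creates a dynamic belt material and sets its color, scale and scroll speed, with visual TrackSpeed separate from transport Speed.
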(event `self.ReceiveTick`
  (params (DeltaSeconds :type "Float (single-precision)"))
  (for _array_element (`PrimitiveComponent.GetOverlappingActors` (`self.Box`) null)
    (cast `/Game/VRE/Core/Character/FPS_VRCharacter` _array_element
      (:`CastFailed`
        (`self.K2_AddActorWorldOffset` _array_element (* (* DeltaSeconds (`self.Speed`)) (`KismetMathLibrary.GetForwardVector` (`SceneComponent.K2_GetComponentRotation` (`self.StaticMesh`)))) false false)
        (if true
          _)))))

(fn `UserConstructionScript`
  (bind _returnvalue (`PrimitiveComponent.CreateDynamicMaterialInstance` (`self.StaticMesh`) 0 "/Game/Library/Materials/MI_BeltWorking.MI_BeltWorking" "None"))
  (`MaterialInstanceDynamic.SetVectorParameterValue` _returnvalue "Color" (`self.Color`))
  (`MaterialInstanceDynamic.SetScalarParameterValue` _returnvalue "XScale" (`self.Scale`))
  (`MaterialInstanceDynamic.SetScalarParameterValue` _returnvalue "XSpeed" (`self.TrackSpeed`)))