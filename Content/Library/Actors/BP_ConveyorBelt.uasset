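; Conveyor belt actor that carries any actor overlapping its box volume along the direction of its arrow component.
; While Speed is non-zero, Tick offsets each overlapping actor by Speed scaled by delta time, without sweep or physics forces.
; SetSpeed changes the rate from outside.
; An unconnected leftover would set the working-belt material and a default speed, but never runs.
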(event `self.ReceiveTick`
  (params (DeltaSeconds :type "Float (single-precision)"))
  (if (not (== (`self.Speed`) 0.0))
    (for _array_element (`PrimitiveComponent.GetOverlappingActors` (`self.Box`) null)
      (`self.K2_AddActorWorldOffset` _array_element (* (* DeltaSeconds (`self.Speed`)) (`KismetMathLibrary.GetForwardVector` (`SceneComponent.K2_GetComponentRotation` (`self.Arrow`)))) false false))))

(event `self.ReceiveBeginPlay`)

(fn `SetSpeed`
  (params (Speed :type "Float (double-precision)"))
  (set `self.Speed` Speed))

(fn `UserConstructionScript`)