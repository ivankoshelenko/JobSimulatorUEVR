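; Quest manager Blueprint that loads the game's quest definitions at startup.
; On BeginPlay it iterates every row name in the DT_Quests data table and appends each found row to its QuestList array.
; A disconnected debug loop, which never runs, would print each quest's name, description, hint and completed flag.
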(event `self.ReceiveBeginPlay`
  (bind _outrownames (`DataTableFunctionLibrary.GetDataTableRowNames` "/Game/Library/Quest/DT_Quests.DT_Quests"))
  (for _array_element _outrownames
    (bind _returnvalue (`|GetDataTableRow` "/Game/Library/Quest/DT_Quests.DT_Quests" _array_element)
      (:`then`
        (`KismetArrayLibrary.Array_Add` (`self.QuestList`) _returnvalue)))))

(fn `UserConstructionScript`)