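; BP_Tablet is a grippable quest tablet that announces the first time it is picked up.
; On grip, an IsHeld guard lets the logic run only while unset, and the flag is never cleared here.
; It plays a 2D sound, then broadcasts OnTabletGrabMessage to every BPI_QuestBus actor and UpdateMessage to every BPI_UpdateDesk widget to update Quest 1.
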(event `VRGripInterface.OnGrip`
  (params (GrippingController :type "GripMotionControllerComponent Object Reference") (GripInformation :type "BPActorGripInformation Structure (by ref)"))
  (if (not (== (`self.IsHeld`) true))
    (`|ExecutionSequence`
      (:`then_0`
        (`GameplayStatics.PlaySound2D` "/Engine/VREditor/Sounds/UI/Enter_Simulate.Enter_Simulate" 1.0 1.0 0.0 null null))
      (:`then_1`
        (set `self.IsHeld` true)
        (bind _outactors (`GameplayStatics.GetAllActorsWithInterface` "/Game/Library/Quest/BPI_QuestBus.BPI_QuestBus_C"))
        (for _array_element _outactors
          (`KismetSystemLibrary.PrintString` "Tablet Grabbed")
          (message `/Game/Library/Quest/BPI_QuestBus.OnTabletGrab` _array_element)))
      (:`then_2`
        (bind _foundwidgets (`WidgetBlueprintLibrary.GetAllWidgetsWithInterface` "/Game/Library/Quest/BPI_UpdateDesk.BPI_UpdateDesk_C"))
        (for _array_element_2 _foundwidgets
          (`KismetSystemLibrary.PrintString` "Quest 1 Updated")
          (message `/Game/Library/Quest/BPI_UpdateDesk.Update` _array_element_2 0))))))

(fn `UserConstructionScript`)