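; BP_Bookshelf is a quest-library bookshelf with labeled signs and book slot collision components.
; On BeginPlay, SetSigns writes the left and right labels to both faces of each sign.
; It then disables collision on a random BookSlots child; the printed name comes from a separate random pick, so may differ.
; Overlap events on slots D1 to D3 only print the overlapping actor and slot name.
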(event `self.ReceiveBeginPlay`
  (bind _outitem (`KismetArrayLibrary.Array_Random` (`SceneComponent.GetChildrenComponents` (`self.Book slots`) false)))
  (`self.SetSigns` (`self.LeftSign`) (`self.RightSign`))
  (`KismetSystemLibrary.PrintString` (`KismetSystemLibrary.GetDisplayName` _outitem))
  (bind _asprimitive_component (cast `PrimitiveComponent` _outitem))
  (`PrimitiveComponent.SetCollisionEnabled` _asprimitive_component "NoCollision"))

(event `self.Book slot d1.OnComponentBeginOverlap`
  (params (OverlappedComponent :type "PrimitiveComponent Object Reference") (OtherActor :type "Actor Object Reference") (OtherComp :type "PrimitiveComponent Object Reference") (OtherBodyIndex :type Integer) (bFromSweep :type Boolean) (SweepResult :type "HitResult Structure (by ref)"))
  (`KismetSystemLibrary.PrintString` (`KismetStringLibrary.Concat_StrStr` (`KismetSystemLibrary.GetDisplayName` OtherActor) " " "D1")))

(event `self.Book slot d2.OnComponentBeginOverlap`
  (params (OverlappedComponent :type "PrimitiveComponent Object Reference") (OtherActor :type "Actor Object Reference") (OtherComp :type "PrimitiveComponent Object Reference") (OtherBodyIndex :type Integer) (bFromSweep :type Boolean) (SweepResult :type "HitResult Structure (by ref)"))
  (`KismetSystemLibrary.PrintString` (`KismetStringLibrary.Concat_StrStr` (`KismetSystemLibrary.GetDisplayName` OtherActor) " " "D2")))

(event `self.Book slot d3.OnComponentBeginOverlap`
  (params (OverlappedComponent :type "PrimitiveComponent Object Reference") (OtherActor :type "Actor Object Reference") (OtherComp :type "PrimitiveComponent Object Reference") (OtherBodyIndex :type Integer) (bFromSweep :type Boolean) (SweepResult :type "HitResult Structure (by ref)"))
  (`KismetSystemLibrary.PrintString` (`KismetStringLibrary.Concat_StrStr` (`KismetSystemLibrary.GetDisplayName` OtherActor) "" "D3")))

(fn `SetSigns`
  (params (LeftSign :type String) (RightSign :type String))
  (bind _returnvalue (`KismetTextLibrary.Conv_StringToText` LeftSign))
  (bind _returnvalue_2 (`KismetTextLibrary.Conv_StringToText` RightSign))
  (`|ExecutionSequence`
    (:`then_0`
      (`TextRenderComponent.K2_SetText` (`self.LeftSignFront`) _returnvalue))
    (:`then_1`
      (`TextRenderComponent.K2_SetText` (`self.LeftSignBack`) _returnvalue))
    (:`then_2`
      (`TextRenderComponent.K2_SetText` (`self.RightSignFront`) _returnvalue_2))
    (:`then_3`
      (`TextRenderComponent.K2_SetText` (`self.RightSignBack`) _returnvalue_2))))

(fn `UserConstructionScript`)